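; Lobby game mode that manages connected players, host map settings, kicking and server travel into the selected map.
; On login it sets up each LobbyPC and spawns a first-person character at a random PlayerStart.
; Joins, respawns, kicks and logouts rebroadcast player info and counts to every controller, then run a readiness check that sets CanWeStart.
; An OnRep on the controller list copies Steam avatars into the game state.
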(event `self.K2_PostLogin`
  (params (NewPlayer :type "PlayerController Object Reference"))
  ;[1 1 1] Initial Lobby Setup - Spawns Player
  (`/Engine/EditorBlueprintResources/ActorMacros.Switch Has Authority`
    (:`Authority`
      (`KismetArrayLibrary.Array_AddUnique` (`self.AllPlayerControllers`) NewPlayer)
      (bind _outactors (`GameplayStatics.GetAllActorsOfClass` "/Script/Engine.PlayerStart"))
      (set `self.SpawnPoints` _outactors)
      (bind _asgame_info_instance (cast `/Game/Networking/Blueprints/AllLevels/GameInfoInstance` (`GameplayStatics.GetGameInstance`)))
      (set `self.ServerName` (`/Game/Networking/Blueprints/AllLevels/GameInfoInstance.ServerName` _asgame_info_instance))
      (set `self.MaxPlayers` (`/Game/Networking/Blueprints/AllLevels/GameInfoInstance.MaxNumPlayers` _asgame_info_instance))
      (bind _aslobby_pc (cast `/Game/Networking/Blueprints/Lobby/LobbyPC` NewPlayer))
      (`/Game/Networking/Blueprints/Lobby/LobbyPC.InitialSetup` _aslobby_pc)
      (`/Game/Networking/Blueprints/Lobby/LobbyPC.SetupLobbyMenu` _aslobby_pc (`self.ServerName`))
      (`/Game/Networking/Blueprints/Lobby/LobbyPC.UpdateLobbySettings` _aslobby_pc (`self.GMMapImage`) (`self.GMMapName`) (`self.DisMapMode`) (`self.GMMapTime`))
      (`self.RespawnPlayer` NewPlayer)
      (`self.EveryoneUpdate`))))

(event `RespawnPlayer`
  (params (PlayerController :type "PlayerController Object Reference"))
  (bind _returnvalue (`Controller.K2_GetPawn` PlayerController))
  (bind _spawnpoints (`self.SpawnPoints`))
  ;[1 1 1] Spawn The Player - Updates Everyones Lobby
  (`/Engine/EditorBlueprintResources/StandardMacros.IsValid` _returnvalue
    (:`Is Valid`
      (`self.K2_DestroyActor` _returnvalue))
    (:`Is Not Valid`
      _))
  (bind _returnvalue_2 (`|SpawnActorFromClass` "/Game/FirstPersonBP/Blueprints/FirstPersonCharacter.FirstPersonCharacter_C" (`self.GetTransform` (`KismetArrayLibrary.Array_Get` _spawnpoints (`KismetMathLibrary.RandomIntegerInRange` 0 (- (`KismetArrayLibrary.Array_Length` _spawnpoints) 1)))) "Undefined" "OverrideRootScale"))
  (`Controller.Possess` PlayerController _returnvalue_2)
  (`self.EveryoneUpdate`))

(event `EveryoneUpdate`
  (bind _allplayercontrollers (`self.AllPlayerControllers`))
  ;[1 1 1] Updates Connected Players Lobby Information
  (bind _output_get (set `self.CurrentPlayers` (`KismetArrayLibrary.Array_Length` (`self.AllPlayerControllers`))))
  (if (not (== _output_get 0))
    (`KismetArrayLibrary.Array_Clear` (`self.ConnectedPlayers`))
    (for _array_element _allplayercontrollers
      (bind _aslobby_pc (cast `/Game/Networking/Blueprints/Lobby/LobbyPC` _array_element))
      (`KismetArrayLibrary.Array_Add` (`self.ConnectedPlayers`) (`/Game/Networking/Blueprints/Gameplay/GameplayPlayerState.PlayerInfo` (cast `/Game/Networking/Blueprints/Gameplay/GameplayPlayerState` (`Controller.PlayerState` _aslobby_pc) :!pure true)))
      (`/Game/Networking/Blueprints/Lobby/LobbyPC.UpdateNumberOfPlayers` _aslobby_pc (`self.CurrentPlayers`) (`self.MaxPlayers`)))
    (`KismetSystemLibrary.Delay` 0.1)
    (for _array_element_2 _allplayercontrollers
      (bind _aslobby_pc_2 (cast `/Game/Networking/Blueprints/Lobby/LobbyPC` _array_element_2))
      (`/Game/Networking/Blueprints/Lobby/LobbyPC.AddPlayerInfo` _aslobby_pc_2 (`self.ConnectedPlayers`)))
    (`self.CannotStartCheck` (`self.ConnectedPlayers`) :!label _label
      (:`CannotStart`
        (`self.CannotStartGame`)))))

(event `CannotStartGame`
  ;[1 1 1] Updates Connected Players Lobby Information
  (goto _label :!via `Break-CannotStart`))

(event `ServerUpdateGameSettings`
  (params (MapImage :type "Texture2D Object Reference") (MapName :type Text) (DisMapMode :type Text) (MapTime :type Text) (LiteralMapName :type Text))
  ;[1 1 1] Server Has Made Changes - Tell Each Client
  (set `self.GMMapImage` MapImage)
  (set `self.GMMapName` MapName)
  (set `self.DisMapMode` DisMapMode)
  (set `self.GMMapTime` MapTime)
  (set `self.GM_LiteralMapName` LiteralMapName)
  (for _array_element (`self.AllPlayerControllers`)
    (bind _aslobby_pc (cast `/Game/Networking/Blueprints/Lobby/LobbyPC` _array_element))
    (`/Game/Networking/Blueprints/Lobby/LobbyPC.UpdateLobbySettings` _aslobby_pc (`self.GMMapImage`) (`self.GMMapName`) (`self.DisMapMode`) (`self.GMMapTime`))))

(event `LaunchGame`
  ;[1 1 1] Launch Game Based On Map
  (bind _asgame_info_instance (cast `/Game/Networking/Blueprints/AllLevels/GameInfoInstance` (`GameplayStatics.GetGameInstance`)))
  (set `/Game/Networking/Blueprints/AllLevels/GameInfoInstance.MainMenu` false _asgame_info_instance)
  (`KismetSystemLibrary.ExecuteConsoleCommand` (`KismetTextLibrary.Conv_TextToString` (`|FormatText` "servertravel /Game/Networking/NetSafeMaps/BuildMaps/{LiteralMapName}" (`self.GM_LiteralMapName`))) (`GameplayStatics.GetPlayerController` 0)))

(event `YouHaveBeenKicked`
  (params (PlayerID :type Integer))
  ;[1 1 1] Kick The Selected Player
  (`/Game/Networking/Blueprints/Lobby/LobbyPC.Kicked` (cast `/Game/Networking/Blueprints/Lobby/LobbyPC` (`KismetArrayLibrary.Array_Get` (`self.AllPlayerControllers`) PlayerID) :!pure true))
  (`self.EveryoneUpdate`))

(event `self.K2_OnLogout`
  (params (ExitingController :type "Controller Object Reference"))
  (bind _allplayercontrollers (`self.AllPlayerControllers`))
  ;[1 1 1] OnLoggout Removes PC and Connected Player Info
  (for (_array_element _array_index) _allplayercontrollers
    (if (== _array_element ExitingController)
      (break)))
  (`KismetArrayLibrary.Array_Remove` _allplayercontrollers _array_index)
  (`KismetArrayLibrary.Array_Remove` (`self.ConnectedPlayers`) _array_index)
  (`KismetArrayLibrary.Array_Remove` (`GameStateBase.PlayerArray` (`GameplayStatics.GetGameState`)) _array_index)
  (`self.EveryoneUpdate`))

(fn `OnRep_AllPlayerControllers`
  (locals (TempAvatars :type "Array of Texture2D Object Reference"))
  (bind _allplayercontrollers (`self.AllPlayerControllers`))
  (`KismetArrayLibrary.Array_Clear` (`local.TempAvatars`))
  (for (_ _array_index) _allplayercontrollers
    (bind _returnvalue (`AdvancedFriendsLibrary.GetSteamFriendAvatar` (`AdvancedSessionsLibrary.GetUniqueNetID` (`KismetArrayLibrary.Array_Get` _allplayercontrollers _array_index)) "SteamAvatar_Large")
      (:`OnSuccess`
        (`KismetArrayLibrary.Array_AddUnique` (`local.TempAvatars`) _returnvalue))))
  (set `/Game/Networking/Blueprints/Gameplay/GameplayGameState.Avatars` (`local.TempAvatars`) (cast `/Game/Networking/Blueprints/Gameplay/GameplayGameState` (`GameplayStatics.GetGameState`) :!pure true)))

(fn `UserConstructionScript`)