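; Training game mode Blueprint that ends the session with a congratulations screen once a score threshold is exceeded.
; On the over-threshold event it adds the widget to the viewport, disables input on the first player's pawn, and switches to UI-only input with a visible cursor.
; It also sets the GameState's GameMode enum, while BeginPlay, Tick and construction just defer to the parent.
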(event `self.ReceiveBeginPlay`
  (`parent.ReceiveBeginPlay`))

(event `self.ReceiveTick`
  (params (DeltaSeconds :type "Float (single-precision)"))
  (`parent.ReceiveTick` DeltaSeconds))

(event `/Game/Networking/Blueprints/Gameplay/GameplayGM.Over Score Threshold`
  (params (`Team That Is Over` :type "/Game/Networking/Blueprints/AllLevels/TeamIdentifier Enum" :default "NewEnumerator0"))
  (bind _returnvalue (`GameplayStatics.GetPlayerController` 0))
  ;[1 1 1] The Dankest Memiest Comennt
  (bind _returnvalue_2 (`|CreateWidget` "/Game/Networking/UI/CongratulationsScreen.CongratulationsScreen_C"))
  (`UserWidget.AddToViewport` _returnvalue_2 99)
  (`self.DisableInput` (`Controller.K2_GetPawn` _returnvalue) _returnvalue)
  (`WidgetBlueprintLibrary.SetInputMode_UIOnlyEx` _returnvalue null "LockAlways")
  (set `PlayerController.bShowMouseCursor` true _returnvalue))

(event `/Game/Networking/Blueprints/Gameplay/GameplayGM.SetGameModeGameState`
  (params (GameState :type "/Game/Networking/Blueprints/Gameplay/GameplayGameState Object Reference"))
  (set `/Game/Networking/Blueprints/Gameplay/GameplayGameState.GameMode` "NewEnumerator3" GameState))

(fn `UserConstructionScript`
  (`parent.UserConstructionScript`))