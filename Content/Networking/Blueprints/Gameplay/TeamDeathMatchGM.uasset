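; Team deathmatch game mode for a networked game, decided by comparing red and blue team scores when time runs out.
; TimedOut passes one of three outcome enums to DisplayWinGame, covering a tie, a red win and a blue win.
; SetGameModeGameState tags the given game state with this mode's enum value.
; BeginPlay, Tick and construction only call the parent, and scoring and timing logic are not in this Blueprint.
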(event `self.ReceiveTick`
  (params (DeltaSeconds :type "Float (single-precision)"))
  (`parent.ReceiveTick` DeltaSeconds))

(event `self.ReceiveBeginPlay`
  (`parent.ReceiveBeginPlay`))

(event `self.TimedOut`
  ;[1 1 1] Game Time Out
  (if (== (`self.RedTeamScore`) (`self.BlueTeamScore`))
    (`self.DisplayWinGame` "NewEnumerator2")
    (elif (> (`self.RedTeamScore`) (`self.BlueTeamScore`))
      (`self.DisplayWinGame` "NewEnumerator0")
      (else
        (`self.DisplayWinGame` "NewEnumerator1")))))

(event `self.SetGameModeGameState`
  (params (GameState :type "/Game/Networking/Blueprints/Gameplay/GameplayGameState Object Reference"))
  (set `/Game/Networking/Blueprints/Gameplay/GameplayGameState.GameMode` "NewEnumerator1" GameState))

(fn `UserConstructionScript`
  (`parent.UserConstructionScript`))