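; Player state for a capture-the-flag mode that keeps per-player gameplay statistics.
; Separate events each add one to flags captured, flag returns or player kills, and a function adds a given amount to the bullets-fired total.
; It only accumulates counters, with no logic on begin play, tick or construction.
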(event `IncreaseNumCaptured`
  (set `self.NumFlagsCaptured` (- (`self.NumFlagsCaptured`) -1)))

(event `FlagReturnIncrease`
  (set `self.FlagReturnsCount` (- (`self.FlagReturnsCount`) -1)))

(event `PlayerKillsIncrease`
  (set `self.PlayerKillCount` (- (`self.PlayerKillCount`) -1)))

(fn `AddBulletsFired`
  (params (Bullets :type Integer))
  (set `self.BulletsFired` (+ Bullets (`self.BulletsFired`))))

(fn `UserConstructionScript`)