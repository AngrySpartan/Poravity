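; Game mode for Infiltration, a round-based flag match where Red and Blue alternate as attackers.
; Timeout or score threshold shows end-round screens, then a timer starts the next round.
; New rounds respawn players, add the attackers' score to their total, swap sides and reset the flag.
; After the last round team scores pick the winner, ties add rounds, and OnRep functions copy state to InfiltrationGameState.
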(event `Swap Attacking Team`
  (params (`Current Attacking Team` :type "/Game/Networking/Blueprints/AllLevels/TeamIdentifier Enum"))
  ;[1 1 1] Swap Attacking Team
  (set `self.AttackingTeam` (select `/Game/Networking/Blueprints/AllLevels/TeamIdentifier` `Current Attacking Team` :`NewEnumerator0` "NewEnumerator1" :`NewEnumerator1` "NewEnumerator0" :`NewEnumerator2` "NewEnumerator0" :!type "/Game/Networking/Blueprints/AllLevels/TeamIdentifier Enum")))

(event `Re Setup Flag`
  ;[1 1 1] Reset The Flag For New Attacking Team
  (bind _outactors (`GameplayStatics.GetAllActorsOfClass` "/Game/FirstPersonBP/Blueprints/Flag/Flag.Flag_C"))
  (bind _item (`KismetArrayLibrary.Array_Get` _outactors))
  (set `/Game/FirstPersonBP/Blueprints/Flag/Flag.OwnerTeam` (`self.AttackingTeam`) _item)
  (`KismetSystemLibrary.Delay` 0.2)
  (`/Game/FirstPersonBP/Blueprints/Flag/Flag.RespawnFlag` _item))

(event `self.ReceiveBeginPlay`
  ;[1 1 1] Parent BeginPlay/Tick
  (`parent.ReceiveBeginPlay`))

(event `self.ReceiveTick`
  (params (DeltaSeconds :type "Float (single-precision)"))
  ;[1 1 1] Parent BeginPlay/Tick
  (`parent.ReceiveTick` DeltaSeconds))

(event `self.SetGameModeGameState`
  (params (GameState :type "/Game/Networking/Blueprints/Gameplay/GameplayGameState Object Reference"))
  ;[1 1 1] Initialize Game Mode in Game State
  (set `/Game/Networking/Blueprints/Gameplay/GameplayGameState.GameMode` "NewEnumerator0" GameState))

(event `Start New Round`
  (bind _attackingteam (`self.AttackingTeam`))
  ;[1 1 1] Starting a new Round
  (if (not (`self.GameOver`))
    (`KismetSystemLibrary.K2_ClearTimer` null "Start New Round")
    (`|ExecutionSequence`
      (:`then_0`
        (`KismetSystemLibrary.Delay` 2.22)
        (`self.Respawn All Players`
          (:`Out`
            (`self.Respawn All Players`))))
      (:`then_1`
        (`KismetSystemLibrary.Delay` (`self.NextRoundDelayHalf`))
        (if (not (`self.GameOver`))
          (switch `/Game/Networking/Blueprints/AllLevels/TeamIdentifier` _attackingteam
            (:`NewEnumerator0`
              (set `self.RedTeamTotalScore` (+ (`self.RedTeamTotalScore`) (`self.RedTeamScore`))))
            (:`NewEnumerator1`
              (set `self.BlueTeamTotalScore` (+ (`self.BlueTeamTotalScore`) (`self.BlueTeamScore`))))
            (:`NewEnumerator2`
              _))
          (`self.Swap Attacking Team` _attackingteam)
          (set `self.GameTimeRemaining` (`self.RoundTime`))
          (`self.Re Setup Flag`)
          (set `self.GameOver` false)
          (`/Engine/EditorBlueprintResources/StandardMacros.IncrementInt` (`self.CurrentRound`)
            (:`  `
              (set `self.EndOfRound` false))))))))

(event `self.TimedOut`
  ;[1 1 1] Game Timed Out Override
  (for _array_element (`self.AllPlayerControllers`)
    (bind _asgameplay_pc (cast `/Game/Networking/Blueprints/Gameplay/GameplayPC` _array_element))
    (`/Game/Networking/Blueprints/Gameplay/GameplayPC.DisplayEndRoundScreen` _asgameplay_pc (`self.NextRoundDelayHalf`))
    (`self.EndOfRoundTime`))
  (if (>= (`self.CurrentRound`) (`self.MaxNumRounds`))
    (`self.Check Scores To Have a Winner`
      (:`New Round Started`
        (set `self.WinAmntNeeded` (- (`self.WinAmntNeeded`) -1))))
    (else
      (`KismetSystemLibrary.K2_SetTimer` null "Start New Round" (`self.NextRoundDelayHalf`)))))

(event `self.Over Score Threshold`
  (params (`Team That Is Over` :type "/Game/Networking/Blueprints/AllLevels/TeamIdentifier Enum" :default "NewEnumerator0"))
  ;[1 1 1] Win Game Override
  (if (> (`self.GameTimeRemaining`) 0.0)
    (for _array_element (`self.AllPlayerControllers`)
      (bind _asgameplay_pc (cast `/Game/Networking/Blueprints/Gameplay/GameplayPC` _array_element))
      (`/Game/Networking/Blueprints/Gameplay/GameplayPC.DisplayEndRoundScreen` _asgameplay_pc (`self.NextRoundDelayHalf`))
      (`self.EndOfRoundTime`))
    (if (>= (`self.CurrentRound`) (`self.MaxNumRounds`))
      (`self.Check Scores To Have a Winner`
        (:`New Round Started`
          (set `self.WinAmntNeeded` (- (`self.WinAmntNeeded`) -1))))
      (else
        (`KismetSystemLibrary.K2_SetTimer` null "Start New Round" (`self.NextRoundDelayHalf`))))))

(event `self.Set Game Time`
  (params (MaxTime :type "Float (single-precision)"))
  ;[1 1 1] Initialize Round Time
  (bind _foundwidgets (`WidgetBlueprintLibrary.GetAllWidgetsOfClass` "/Game/Networking/UI/Gameplay/Gameplay_Main_UI.Gameplay_Main_UI_C"))
  (`Widget.SetVisibility` (`/Game/Networking/UI/Gameplay/Gameplay_Main_UI.TimeLeft` (`KismetArrayLibrary.Array_Get` _foundwidgets)) "Visible")
  (bind _output_get (set `self.RoundTime` MaxTime))
  (set `self.GameTimeRemaining` _output_get))

(event `EndOfRoundTime`
  ;[1 1 1] Initialize Round Time
  (bind _foundwidgets (`WidgetBlueprintLibrary.GetAllWidgetsOfClass` "/Game/Networking/UI/Gameplay/Gameplay_Main_UI.Gameplay_Main_UI_C"))
  (`Widget.SetVisibility` (`/Game/Networking/UI/Gameplay/Gameplay_Main_UI.TimeLeft` (`KismetArrayLibrary.Array_Get` _foundwidgets)) "Hidden")
  (set `self.GameTimeRemaining` 100.0)
  (set `self.EndOfRound` true))

(fn `OnRep_AttackingTeam`
  (bind _asinfiltration_game_state (cast `/Game/Networking/Blueprints/Gameplay/InfiltrationGameState` (`GameplayStatics.GetGameState`)))
  (set `/Game/Networking/Blueprints/Gameplay/InfiltrationGameState.AttackingTeam` (`self.AttackingTeam`) _asinfiltration_game_state))

(fn `OnRep_BlueTeamRoundScore`
  (bind _asinfiltration_game_state (cast `/Game/Networking/Blueprints/Gameplay/InfiltrationGameState` (`GameplayStatics.GetGameState`)))
  (set `/Game/Networking/Blueprints/Gameplay/InfiltrationGameState.BlueTeamTotalScore` (`self.BlueTeamTotalScore`) _asinfiltration_game_state))

(fn `OnRep_CurrentRound`
  (bind _asinfiltration_game_state (cast `/Game/Networking/Blueprints/Gameplay/InfiltrationGameState` (`GameplayStatics.GetGameState`)))
  (set `/Game/Networking/Blueprints/Gameplay/InfiltrationGameState.CurrentRound` (`self.CurrentRound`) _asinfiltration_game_state))

(fn `OnRep_RedTeamRoundScore`
  (bind _asinfiltration_game_state (cast `/Game/Networking/Blueprints/Gameplay/InfiltrationGameState` (`GameplayStatics.GetGameState`)))
  (set `/Game/Networking/Blueprints/Gameplay/InfiltrationGameState.RedTeamTotalScore` (`self.RedTeamTotalScore`) _asinfiltration_game_state))

(fn `OnRep_StartNewRoundTimer`)

(fn `UserConstructionScript`
  (`parent.UserConstructionScript`))