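; Team safe zone barrier actor that blocks characters of one team, apparently to keep enemies out of a base.
; When a first-person character overlaps the Cube, its Pawn response becomes Block if the character's team matches PlayerTeam, otherwise Overlap.
; A Box overlap resets the Cube to Overlap; this collision state is shared by all pawns.
; The construction script colors the Cube opposite to PlayerTeam, so PlayerTeam denotes the blocked team.
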(event `self.Cube.OnComponentBeginOverlap`
  (params (OverlappedComponent :type "PrimitiveComponent Object Reference") (OtherActor :type "Actor Object Reference") (OtherComp :type "PrimitiveComponent Object Reference") (OtherBodyIndex :type Integer) (bFromSweep :type Boolean) (SweepResult :type "HitResult Structure (by ref)"))
  (bind _asfirst_person_character (cast `/Game/FirstPersonBP/Blueprints/FirstPersonCharacter` OtherActor))
  (`self.PreventEnemyInfiltration` _asfirst_person_character))

(event `PreventEnemyInfiltration`
  (params (CharacterRef :type "/Game/FirstPersonBP/Blueprints/FirstPersonCharacter Object Reference"))
  (bind _cube (`self.Cube`))
  (if (== (`self.PlayerTeam`) (`/Game/FirstPersonBP/Blueprints/FirstPersonCharacter.Team` CharacterRef))
    (`PrimitiveComponent.SetCollisionResponseToChannel` _cube "ECC_Pawn" "ECR_Block")
    (else
      (`PrimitiveComponent.SetCollisionResponseToChannel` _cube "ECC_Pawn" "ECR_Overlap"))))

(event `self.Box.OnComponentBeginOverlap`
  (params (OverlappedComponent :type "PrimitiveComponent Object Reference") (OtherActor :type "Actor Object Reference") (OtherComp :type "PrimitiveComponent Object Reference") (OtherBodyIndex :type Integer) (bFromSweep :type Boolean) (SweepResult :type "HitResult Structure (by ref)"))
  (cast `/Game/FirstPersonBP/Blueprints/FirstPersonCharacter` OtherActor)
  (`self.ResetCubeCollision`))

(event `ResetCubeCollision`
  (`PrimitiveComponent.SetCollisionResponseToChannel` (`self.Cube`) "ECC_Pawn" "ECR_Overlap"))

(fn `UserConstructionScript`
  (bind _cube (`self.Cube`))
  (switch `/Game/Networking/Blueprints/AllLevels/TeamIdentifier` (`self.PlayerTeam`)
    (:`NewEnumerator0`
      (`PrimitiveComponent.SetMaterial` _cube 0 "/Game/Blueprints/Components/Created_Mats/BaseDefenseBlue.BaseDefenseBlue"))
    (:`NewEnumerator1`
      (`PrimitiveComponent.SetMaterial` _cube 0 "/Game/Blueprints/Components/Created_Mats/BaseDefenseRed.BaseDefenseRed"))))