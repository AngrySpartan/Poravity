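; Teleporter entrance actor that sends the first-person character to a linked exit (TelExit) on overlapping its trigger box.
; If InvertGravity is set and the character's gravity is inverted, it first calls the gravity component's OnSpawnFlip.
; It then teleports the character along the exit arrow, matches control rotation to that arrow and launches them forward.
; AmountToMoveUpBy scales both the exit offset and launch velocity.
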(event `self.ReceiveBeginPlay`)

(event `self.Box.OnComponentBeginOverlap`
  (params (OverlappedComponent :type "PrimitiveComponent Object Reference") (OtherActor :type "Actor Object Reference") (OtherComp :type "PrimitiveComponent Object Reference") (OtherBodyIndex :type Integer) (bFromSweep :type Boolean) (SweepResult :type "HitResult Structure (by ref)"))
  (bind _telexit (`self.TelExit`))
  (bind _arrow (`/Game/Blueprints/TeleporterExit.Arrow` _telexit))
  (bind _returnvalue (* (`SceneComponent.GetForwardVector` _arrow) (`self.AmountToMoveUpBy`)))
  (bind _asfirst_person_character (cast `/Game/FirstPersonBP/Blueprints/FirstPersonCharacter` OtherActor))
  (if (and (`/Game/FirstPersonBP/Blueprints/FirstPersonCharacter.bIsGravityInverted` _asfirst_person_character) (`self.InvertGravity`))
    (`/Game/FirstPersonBP/Blueprints/ActorComponents/GravityComponent.OnSpawnFlip` (`/Game/FirstPersonBP/Blueprints/FirstPersonCharacter.GravityComponent` _asfirst_person_character)))
  (`self.K2_SetActorLocation` _asfirst_person_character (+ (`SceneComponent.K2_GetComponentLocation` (`/Game/Blueprints/TeleporterExit.Box` _telexit)) _returnvalue) false true)
  (`Controller.SetControlRotation` (cast `/Game/Networking/Blueprints/Gameplay/GameplayPC` (`Pawn.GetController` _asfirst_person_character) :!pure true) (`SceneComponent.K2_GetComponentRotation` _arrow))
  (`Character.LaunchCharacter` _asfirst_person_character _returnvalue true true))

(fn `UserConstructionScript`)