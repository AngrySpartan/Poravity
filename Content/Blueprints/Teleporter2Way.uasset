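; Two-way teleporter actor that sends a first-person character entering its Box trigger to the teleporter referenced by TwoWay.
; The character lands at that teleporter's Cylinder, offset along its Arrow's forward vector by AmountToMoveUpBy.
; If SetRotation is on, the GameplayPC's control rotation snaps to the Arrow.
; The character is then launched along the Arrow, reusing AmountToMoveUpBy as launch speed and overriding existing velocity.
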(event `self.ReceiveBeginPlay`)

(event `self.Box.OnComponentBeginOverlap`
  (params (OverlappedComponent :type "PrimitiveComponent Object Reference") (OtherActor :type "Actor Object Reference") (OtherComp :type "PrimitiveComponent Object Reference") (OtherBodyIndex :type Integer) (bFromSweep :type Boolean) (SweepResult :type "HitResult Structure (by ref)"))
  (bind _twoway (`self.TwoWay`))
  (bind _arrow (`/Game/Blueprints/Teleporter2Way.Arrow` _twoway))
  (bind _returnvalue (* (`SceneComponent.GetForwardVector` _arrow) (`self.AmountToMoveUpBy`)))
  (bind _asfirst_person_character (cast `/Game/FirstPersonBP/Blueprints/FirstPersonCharacter` OtherActor))
  (`self.K2_SetActorLocation` _asfirst_person_character (+ (`SceneComponent.K2_GetComponentLocation` (`/Game/Blueprints/Teleporter2Way.Cylinder` _twoway)) _returnvalue) false true)
  (if (`self.SetRotation`)
    (`Controller.SetControlRotation` (cast `/Game/Networking/Blueprints/Gameplay/GameplayPC` (`Pawn.GetController` _asfirst_person_character) :!pure true) (`SceneComponent.K2_GetComponentRotation` _arrow)))
  (`Character.LaunchCharacter` _asfirst_person_character _returnvalue true true))

(fn `UserConstructionScript`)