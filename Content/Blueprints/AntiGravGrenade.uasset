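; Anti-gravity grenade projectile that damages and suspends enemy characters and target dummies.
; The server sets projectile gravity from the thrower's inversion state, then detonates on a delay or when the projectile stops.
; Detonation spawns a timeline-scaled ZeroGravityZone, flashes a hit marker and lifts sphere-overlap victims via LerpActorComponent, freezing characters in Flying mode.
; When the timeline finishes, it restores their gravity and movement, respecting inverted gravity, and destroys itself.
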(event `self.ProjectileMovement.OnProjectileStop`
  (params (ImpactResult :type "HitResult Structure (by ref)"))
  ;[1 1 1] Affects Bounciness
  (`/Engine/EditorBlueprintResources/ActorMacros.Switch Has Authority`
    (:`Authority`
      (`self.ProjectileBounce`)
      (`KismetSystemLibrary.K2_ClearTimer` null "ProjectileBounce"))))

(event `self.ReceiveBeginPlay`
  (bind _projectilemovement (`self.ProjectileMovement`))
  (`/Engine/EditorBlueprintResources/ActorMacros.Switch Has Authority`
    (:`Authority`
      (set `ProjectileMovementComponent.InitialSpeed` (`self.InitialSpeed`) (`self.ProjectileMovement`))
      (bind _asfirst_person_character (cast `/Game/FirstPersonBP/Blueprints/FirstPersonCharacter` (`self.Instigator`)))
      (bind _output_get (set `self.MyCharacter` _asfirst_person_character))
      (set `self.MaxJumpHeight` (`CharacterMovementComponent.GetMaxJumpHeight` (`Character.CharacterMovement` _asfirst_person_character)))
      (if (`/Game/FirstPersonBP/Blueprints/FirstPersonCharacter.bIsGravityInverted` _output_get)
        (set `ProjectileMovementComponent.ProjectileGravityScale` -1.0 _projectilemovement)
        (else
          (set `ProjectileMovementComponent.ProjectileGravityScale` 1.0 _projectilemovement)))
      (`PrimitiveComponent.AddImpulseAtLocation` (`self.StaticMesh`) (* (`self.Impulse to Apply`) (`self.GetVelocity` _output_get)) (`self.K2_GetActorLocation`) "None")
      (`KismetSystemLibrary.K2_SetTimer` null "ProjectileBounce" (`self.ExplosionDelay`)))))

(event `ProjectileBounce`
  (bind _mycharacter (`self.MyCharacter`))
  (bind _staticmesh (`self.StaticMesh`))
  (bind _ownerteam (`self.OwnerTeam`))
  (`SceneComponent.SetVisibility` _staticmesh false false)
  (`PrimitiveComponent.SetCollisionEnabled` _staticmesh "NoCollision")
  (`|ExecutionSequence`
    (:`then_0`
      (bind _returnvalue (`|SpawnActorFromClass` "/Game/FirstPersonBP/Blueprints/GravityManipulators/ZeroGravityZone.ZeroGravityZone_C" (`KismetMathLibrary.MakeTransform` (`self.K2_GetActorLocation`) (`self.K2_GetActorRotation`) (0.0 0.0 0.0)) "Undefined" "OverrideRootScale" _mycharacter true _mycharacter))
      (bind (_direction _scalelerptime) (`Timeline|ZeroGScaler` :!via `PlayFromStart`)
        (:`Update`
          (`self.SetActorScale3D` _returnvalue (`KismetMathLibrary.VInterpTo_Constant` (0.0 0.0 0.0) (0.5 0.5 0.5) _scalelerptime 1.0)))
        (:`Finished`
          (for _array_element (`self.PlayerCharacters`)
            (bind _asfirst_person_character (cast `/Game/FirstPersonBP/Blueprints/FirstPersonCharacter` _array_element)
              (:`then`
                (if (not (== (`self.OwnerTeam`) (`/Game/FirstPersonBP/Blueprints/FirstPersonCharacter.Team` _asfirst_person_character)))
                  (if (`/Game/FirstPersonBP/Blueprints/FirstPersonCharacter.bIsGravityInverted` _asfirst_person_character)
                    (bind _charactermovement (`Character.CharacterMovement` _asfirst_person_character))
                    (set `CharacterMovementComponent.GravityScale` -1.0 _charactermovement)
                    (set `CharacterMovementComponent.JumpZVelocity` -450.0 _charactermovement)
                    (else
                      (set `CharacterMovementComponent.GravityScale` 1.0 _charactermovement)
                      (set `CharacterMovementComponent.JumpZVelocity` 450.0 _charactermovement)))
                  (set `CharacterMovementComponent.AirControl` 0.075 _charactermovement)
                  (`CharacterMovementComponent.SetMovementMode` _charactermovement "MOVE_Falling" 0)))
              (:`CastFailed`
                (bind _asdummy_target (cast `/Game/Mannequin/DummyTarget` _array_element))
                (`PrimitiveComponent.SetEnableGravity` (`/Game/Mannequin/DummyTarget.Col` _asdummy_target) true))))
          (`self.K2_DestroyActor`))))
    (:`then_1`
      (bind _outactors (`KismetSystemLibrary.SphereOverlapActors` (`self.K2_GetActorLocation`) (`self.ZeroGRadiusTrace`) (`self.ObjectTypeArray`)))
      (`|ExecutionSequence`
        (:`then_0`
          (set `self.BreakHitMarker` false)
          (for _array_element_2 _outactors
            (bind _asfirst_person_character_2 (cast `/Game/FirstPersonBP/Blueprints/FirstPersonCharacter` _array_element_2)
              (:`then`
                (if (!= (`/Game/FirstPersonBP/Blueprints/FirstPersonCharacter.Team` _asfirst_person_character_2) _ownerteam)
                  (set `self.BreakHitMarker` true :!label _label)
                  (break)))
              (:`CastFailed`
                (cast `/Game/Mannequin/DummyTarget` _array_element_2)
                (goto _label))))
          (if (`self.BreakHitMarker`)
            (`/Game/FirstPersonBP/Blueprints/GunTesting/GunBaseComponent.FlashHitMarkerLoc` (`/Game/FirstPersonBP/Blueprints/FirstPersonCharacter.GunBaseComponent` (cast `/Game/FirstPersonBP/Blueprints/FirstPersonCharacter` (`self.Instigator`) :!pure true)))))
        (:`then_1`
          (bind _output_get (set `self.PlayerCharacters` _outactors))
          (for _array_element_3 _output_get
            (bind _asfirst_person_character_3 (cast `/Game/FirstPersonBP/Blueprints/FirstPersonCharacter` _array_element_3)
              (:`then`
                (bind _team (`/Game/FirstPersonBP/Blueprints/FirstPersonCharacter.Team` _asfirst_person_character_3))
                (if (not (== _ownerteam _team))
                  (set `CharacterMovementComponent.JumpZVelocity` 0.0 (`Character.CharacterMovement` _asfirst_person_character_3))
                  (if (`/Game/FirstPersonBP/Blueprints/FirstPersonCharacter.bIsGravityInverted` _asfirst_person_character_3)
                    (bind _lerpactorcomponent (`/Game/FirstPersonBP/Blueprints/FirstPersonCharacter.LerpActorComponent` _asfirst_person_character_3))
                    (bind _returnvalue_2 (`self.K2_GetActorLocation` _asfirst_person_character_3))
                    (`/Game/FirstPersonBP/Blueprints/ActorComponents/LerpActorComponent.StartLerp` _lerpactorcomponent _returnvalue_2 (+ _returnvalue_2 (0.0 0.0 -333.0)) 2.5)
                    (else
                      (`/Game/FirstPersonBP/Blueprints/ActorComponents/LerpActorComponent.StartLerp` _lerpactorcomponent _returnvalue_2 (+ _returnvalue_2 (0.0 0.0 333.0)) 2.5)))
                  (`/Game/FirstPersonBP/Blueprints/ActorComponents/HealthComponent.OnTakeDamage` (`/Game/FirstPersonBP/Blueprints/FirstPersonCharacter.PlayerHealthComponent` _asfirst_person_character_3) 15.0 _team (0.0 0.0 0.0) null false)))
              (:`CastFailed`
                (bind _asdummy_target_2 (cast `/Game/Mannequin/DummyTarget` _array_element_3))
                (if (not (== _ownerteam (`/Game/Mannequin/DummyTarget.DummyTeam` _asdummy_target_2)))
                  (bind _col (`/Game/Mannequin/DummyTarget.Col` _asdummy_target_2))
                  (`PrimitiveComponent.SetEnableGravity` _col false)
                  (bind _returnvalue_3 (`SceneComponent.K2_GetComponentLocation` _col))
                  (`/Game/FirstPersonBP/Blueprints/ActorComponents/LerpActorComponent.StartLerp` (`/Game/Mannequin/DummyTarget.LerpActorComponent` _asdummy_target_2) _returnvalue_3 (+ _returnvalue_3 (0.0 0.0 250.0)) 3.0)
                  (`/Game/FirstPersonBP/Blueprints/ActorComponents/HealthComponent.OnTakeDamage` (`/Game/Mannequin/DummyTarget.DummyHealthComponent` _asdummy_target_2) 10.0 "NewEnumerator2" (0.0 0.0 0.0) null false)))))
          (for _array_element_4 (`self.PlayerCharacters`)
            (bind _asfirst_person_character_4 (cast `/Game/FirstPersonBP/Blueprints/FirstPersonCharacter` _array_element_4))
            (if (not (== (`self.OwnerTeam`) (`/Game/FirstPersonBP/Blueprints/FirstPersonCharacter.Team` _asfirst_person_character_4)))
              (bind _charactermovement_2 (`Character.CharacterMovement` _asfirst_person_character_4))
              (set `MovementComponent.Velocity` (0.0 0.0 0.0) _charactermovement_2)
              (`CharacterMovementComponent.SetMovementMode` _charactermovement_2 "MOVE_Flying" 0)
              (set `CharacterMovementComponent.AirControl` 0.0 _charactermovement_2))))))))

(fn `UserConstructionScript`)