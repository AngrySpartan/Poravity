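; One-shot spawner actor that produces a pickup of a configurable class after a respawn delay.
; SetupForSpawn starts a non-looping timer of RespawnTime that calls SpawnPickup.
; SpawnPickup spawns PickupType at the spawner's transform, passing ScaleSize and AdditionalArgument into the new actor.
; It then applies ScaleSize as a uniform scale to the pickup and destroys the spawner.
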(event `SetupForSpawn`
  (`KismetSystemLibrary.K2_SetTimerDelegate` (delegate `SpawnPickup`) (`self.RespawnTime`)))

(event `SpawnPickup`
  (bind _scalesize (`self.ScaleSize`))
  (bind _returnvalue (`|SpawnActorFromClass` (`self.PickupType`) (`self.GetTransform`) "Undefined" "OverrideRootScale" null (`self.ScaleSize`) (`self.AdditionalArgument`)))
  (`self.SetActorScale3D` _returnvalue (`KismetMathLibrary.MakeVector` _scalesize _scalesize _scalesize))
  (`self.K2_DestroyActor`))

(fn `UserConstructionScript`)