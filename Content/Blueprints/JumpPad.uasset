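; JumpPad is a Blueprint that launches the first-person character when it overlaps the JumpCollision component.
; The launch velocity is rotated by the Arrow component's world rotation and overrides the character's existing velocity on all axes.
; A DoOnce gate blocks retriggering until a short delay has passed, after which the pad plays its sound, spawns a smoke emitter and resets the gate.
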(event `self.JumpCollision.OnComponentBeginOverlap`
  (params (OverlappedComponent :type "PrimitiveComponent Object Reference") (OtherActor :type "Actor Object Reference") (OtherComp :type "PrimitiveComponent Object Reference") (OtherBodyIndex :type Integer) (bFromSweep :type Boolean) (SweepResult :type "HitResult Structure (by ref)"))
  (bind _asfirst_person_character (cast `/Game/FirstPersonBP/Blueprints/FirstPersonCharacter` OtherActor))
  (`/Engine/EditorBlueprintResources/StandardMacros.DoOnce` false :!label _label
    (:`Completed`
      (`Character.LaunchCharacter` _asfirst_person_character (`KismetMathLibrary.GreaterGreater_VectorRotator` (`self.LaunchVelocity`) (`SceneComponent.K2_GetComponentRotation` (`self.Arrow`))) true true)
      (`KismetSystemLibrary.Delay` 0.2)
      (`GameplayStatics.PlaySoundAtLocation` "/Game/Audio/JumpPad.JumpPad" (`SceneComponent.K2_GetComponentLocation` (`self.Launch_Pad`)))
      (`GameplayStatics.SpawnEmitterAtLocation` "/Game/StarterContent/Particles/P_Smoke.P_Smoke")
      (goto _label :!via `Reset`))))

(fn `UserConstructionScript`)