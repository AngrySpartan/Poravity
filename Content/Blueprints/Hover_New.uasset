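; Hover scene component that floats its owning actor above surfaces using physics forces.
; On BeginPlay it enables physics simulation and sets linear and angular damping on the owner's first primitive component.
; A looping timer, rather than Tick, traces downward from the component.
; On a hit it pushes that primitive along the surface normal, blending from HoverForce to AntiHoverForce as distance approaches RayDistance.
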(event `self.ReceiveBeginPlay`
  (bind _output_get (set `self.PrimitiveComponent` (`KismetArrayLibrary.Array_Get` (`Actor.K2_GetComponentsByClass` (`self.GetOwner`) "/Script/Engine.PrimitiveComponent"))))
  (`PrimitiveComponent.SetSimulatePhysics` _output_get true)
  (`KismetSystemLibrary.K2_SetTimer` null "DoTheFloatyStuff" 0.05 true)
  (`PrimitiveComponent.SetLinearDamping` (`self.PrimitiveComponent`) (`self.LinearDamping`))
  (`PrimitiveComponent.SetAngularDamping` (`self.PrimitiveComponent`) (`self.AngularDamping`)))

(event `DoTheFloatyStuff`
  (bind _returnvalue (`self.K2_GetComponentLocation`))
  (bind (_outhit _returnvalue_2) (`KismetSystemLibrary.LineTraceSingle` _returnvalue (- _returnvalue (`KismetMathLibrary.MakeVector` 0.0 0.0 (`self.RayDistance`))) "TraceTypeQuery1" true))
  (if _returnvalue_2
    (bind (_bblockinghit _binitialoverlap _time _location _impactpoint _normal _impactnormal) (`GameplayStatics.BreakHitResult` _outhit))
    (`PrimitiveComponent.AddForce` (`self.PrimitiveComponent`) (* _impactnormal (`KismetMathLibrary.Lerp` (`self.HoverForce`) (`self.Anti-HoverForce`) (/ (`KismetMathLibrary.VSize` (- _location (`self.K2_GetComponentLocation`))) (`self.RayDistance`)))) "None" false)))