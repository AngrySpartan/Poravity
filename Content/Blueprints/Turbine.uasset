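; Turbine is a hazard actor with four spinning blades that kill the first-person player on contact.
; On BeginPlay its RotatingMovement component spins the Turbine component at the Rotation variable's rate, and a turbine sound spawns at the actor's location.
; Each blade's hit event calls Kill Player, which casts to FirstPersonCharacter and deals massive damage through its PlayerHealthComponent.
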(event `self.ReceiveBeginPlay`
  (bind _rotatingmovement (`self.RotatingMovement`))
  (`MovementComponent.SetUpdatedComponent` _rotatingmovement (`self.Turbine`))
  (set `RotatingMovementComponent.RotationRate` (`self.Rotation`) _rotatingmovement)
  (`GameplayStatics.SpawnSoundAtLocation` "/Game/Audio/Turbine_Cue.Turbine_Cue" (`self.K2_GetActorLocation`)))

(event `self.ReceiveActorBeginOverlap`
  (params (OtherActor :type "Actor Object Reference")))

(event `self.Blade_1.OnComponentHit`
  (params (HitComponent :type "PrimitiveComponent Object Reference") (OtherActor :type "Actor Object Reference") (OtherComp :type "PrimitiveComponent Object Reference") (NormalImpulse :type "Vector Structure") (Hit :type "HitResult Structure (by ref)"))
  (`self.Kill Player` OtherActor))

(event `self.Blade_2.OnComponentHit`
  (params (HitComponent :type "PrimitiveComponent Object Reference") (OtherActor :type "Actor Object Reference") (OtherComp :type "PrimitiveComponent Object Reference") (NormalImpulse :type "Vector Structure") (Hit :type "HitResult Structure (by ref)"))
  (`self.Kill Player` OtherActor))

(event `self.Blade_3.OnComponentHit`
  (params (HitComponent :type "PrimitiveComponent Object Reference") (OtherActor :type "Actor Object Reference") (OtherComp :type "PrimitiveComponent Object Reference") (NormalImpulse :type "Vector Structure") (Hit :type "HitResult Structure (by ref)"))
  (`self.Kill Player` OtherActor))

(event `self.Blade_4.OnComponentHit`
  (params (HitComponent :type "PrimitiveComponent Object Reference") (OtherActor :type "Actor Object Reference") (OtherComp :type "PrimitiveComponent Object Reference") (NormalImpulse :type "Vector Structure") (Hit :type "HitResult Structure (by ref)"))
  (`self.Kill Player` OtherActor))

(fn `UserConstructionScript`)