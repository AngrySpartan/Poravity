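; DeathVolume is a kill zone that kills first-person characters and resets flags that enter it.
; On overlap, a character's valid Flag is respawned, then its health component takes damage equal to twice current health, with a fixed team and the volume's owner as instigator.
; A Flag overlapping directly is also respawned.
; The construction script gives the collision component a dynamic fire material instance.
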(event `self.CollisionComponent.OnComponentBeginOverlap`
  (params (OverlappedComponent :type "PrimitiveComponent Object Reference") (OtherActor :type "Actor Object Reference") (OtherComp :type "PrimitiveComponent Object Reference") (OtherBodyIndex :type Integer) (bFromSweep :type Boolean) (SweepResult :type "HitResult Structure (by ref)"))
  (bind _asfirst_person_character (cast `/Game/FirstPersonBP/Blueprints/FirstPersonCharacter` OtherActor)
    (:`then`
      (bind _flag (`/Game/FirstPersonBP/Blueprints/FirstPersonCharacter.Flag` _asfirst_person_character))
      (`/Engine/EditorBlueprintResources/StandardMacros.IsValid` _flag
        (:`Is Valid`
          (`/Game/FirstPersonBP/Blueprints/Flag/Flag.RespawnFlag` _flag))
        (:`Is Not Valid`
          _))
      (bind _playerhealthcomponent (`/Game/FirstPersonBP/Blueprints/FirstPersonCharacter.PlayerHealthComponent` _asfirst_person_character))
      (`/Game/FirstPersonBP/Blueprints/ActorComponents/HealthComponent.OnTakeDamage` _playerhealthcomponent (* 2 (`/Game/FirstPersonBP/Blueprints/ActorComponents/HealthComponent.CurHealth` _playerhealthcomponent)) "NewEnumerator2" (0.0 0.0 0.0) (`self.GetOwner`)))
    (:`CastFailed`
      (bind _asflag (cast `/Game/FirstPersonBP/Blueprints/Flag/Flag` OtherActor))
      (`/Game/FirstPersonBP/Blueprints/Flag/Flag.RespawnFlag` _asflag))))

(fn `UserConstructionScript`
  (`PrimitiveComponent.CreateDynamicMaterialInstance` (`self.CollisionComponent`) 0 "/Game/AvdMagick/Materials/M_ky_fire01_4x8.M_ky_fire01_4x8"))