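; Spike trap actor that repeatedly thrusts out along its up vector and damages the first-person player.
; A timeline lerps the actor between its start and a LaunchingForce offset, with a ReverseReverse macro alternating forward and backward playback.
; Timeline event tracks play the spike sound and toggle the hit box on then immediately off.
; Box overlap deals heavy damage through the character's health component; the VectorAddition macro is unused.
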(event `self.ReceiveTick`
  (params (DeltaSeconds :type "Float (single-precision)")))

(event `self.ReceiveBeginPlay`
  (bind _box (`self.Box`))
  (`PrimitiveComponent.SetCollisionEnabled` (`self.Box`) "NoCollision")
  (bind _output_get (set `self.InitialLocation` (`self.K2_GetActorLocation`)))
  (set `self.DestinationLocation` (+ _output_get (* (`self.GetActorUpVector`) (`self.LaunchingForce`))))
  (bind (_direction _animationtime) (`Timeline|Timeline_0` :!label _label)
    (:`Update`
      (`self.K2_SetActorLocation` (`KismetMathLibrary.VLerp` (`self.InitialLocation`) (`self.DestinationLocation`) _animationtime)))
    (:`Finished`
      (`self.TimelineFinished`))
    (:`SoundEffect`
      (`GameplayStatics.PlaySoundAtLocation` "/Game/Audio/SpikeTrap_Cue.SpikeTrap_Cue" (`self.K2_GetActorLocation`)))
    (:`SpikeCollision`
      (`PrimitiveComponent.SetCollisionEnabled` _box "QueryAndPhysics")
      (`PrimitiveComponent.SetCollisionEnabled` _box "NoCollision"))))

(event `TimelineFinished`
  (`self.ReverseReverse`
    (:`then`
      (goto _label :!via `PlayFromStart`))
    (:`then2`
      (goto _label :!via `ReverseFromEnd`))))

(event `self.Box.OnComponentBeginOverlap`
  (params (OverlappedComponent :type "PrimitiveComponent Object Reference") (OtherActor :type "Actor Object Reference") (OtherComp :type "PrimitiveComponent Object Reference") (OtherBodyIndex :type Integer) (bFromSweep :type Boolean) (SweepResult :type "HitResult Structure (by ref)"))
  (bind _asfirst_person_character (cast `/Game/FirstPersonBP/Blueprints/FirstPersonCharacter` OtherActor))
  (`/Game/FirstPersonBP/Blueprints/ActorComponents/HealthComponent.OnTakeDamage` (`/Game/FirstPersonBP/Blueprints/FirstPersonCharacter.PlayerHealthComponent` _asfirst_person_character) 500.0 "NewEnumerator2" (0.0 0.0 0.0) (`self.GetOwner`)))

(fn `UserConstructionScript`)