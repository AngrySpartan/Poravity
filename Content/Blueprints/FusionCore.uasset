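; Destructible fusion core that blinks and explodes, damaging its surroundings and shaking nearby cameras before destroying itself.
; Incoming radial damage feeds its health component, and a dynamic material shifts from blue toward red as health drops.
; A one-shot timeline drives the warning blink and sound, then detonates.
; The authority applies falloff damage credited to the recent damager, who separately takes distance-tiered damage through a sphere overlap.
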(event `self.ReceiveRadialDamage`
  (params (DamageReceived :type "Float (single-precision)") (DamageType :type "DamageType Object Reference") (Origin :type "Vector Structure") (HitInfo :type "HitResult Structure (by ref)") (InstigatedBy :type "Controller Object Reference") (DamageCauser :type "Actor Object Reference"))
  ;[1 1 1] Receive Radial Damage
  (`/Game/FirstPersonBP/Blueprints/ActorComponents/HealthComponent.OnTakeDamage` (`self.FusionCoreHealth`) DamageReceived "NewEnumerator2" (0.0 0.0 0.0) DamageCauser true))

(event `ExplodingCore`
  ;[1 1 1] Changes Color of Material
  (`/Engine/EditorBlueprintResources/StandardMacros.DoOnce` false
    (:`Completed`
      (bind (_direction _newtrack_1) (`Timeline|BlinkingLight` :!via `PlayFromStart`)
        (:`Update`
          (`self.ReplicateBlink` _newtrack_1))
        (:`Finished`
          (`self.Explodee`))
        (:`PlayExplosionSound`
          (`self.ReplicatedSound` "/Game/Audio/FusionExplosion.FusionExplosion"))))))

(event `Explodee`
  (bind _returnvalue (`self.K2_GetActorLocation`))
  (bind _recentdamager (`/Game/FirstPersonBP/Blueprints/ActorComponents/FusionCoreHealth.RecentDamager` (`self.FusionCoreHealth`)))
  ;[1 1 1] Changes Color of Material
  (set `self.Exploding` true)
  (`/Engine/EditorBlueprintResources/ActorMacros.Switch Has Authority`
    (:`Authority`
      (`self.ReplicatedEmitter` "/Game/StarterContent/Particles/P_Explosion.P_Explosion" "/Game/StarterContent/Audio/Explosion_Cue.Explosion_Cue")
      (`GameplayStatics.ApplyRadialDamageWithFalloff` :`BaseDamage` (`self.BaseDamage`) :`MinimumDamage` (`self.MinDamage`) :`Origin` _returnvalue :`DamageInnerRadius` 200.0 :`DamageOuterRadius` 500.0 :`DamageFalloff` 1.0 :`DamageTypeClass` "/Script/Engine.DamageType" :`DamageCauser` _recentdamager)
      (bind _outactors (`KismetSystemLibrary.SphereOverlapActors` _returnvalue 500.0 (`|MakeArray` "ObjectTypeQuery3" :!type "EObjectTypeQuery Enum")))
      (for _array_element _outactors
        (if (== _array_element _recentdamager)
          (bind _returnvalue_2 (`KismetMathLibrary.VSize` (- (`self.K2_GetActorLocation` _array_element) _returnvalue)))
          (`/Game/FirstPersonBP/Blueprints/ActorComponents/HealthComponent.OnTakeDamage` (`self.GetComponentByClass` _array_element "/Game/FirstPersonBP/Blueprints/ActorComponents/HealthComponent.HealthComponent_C") (select `bool` (>= _returnvalue_2 400.0) :`false` (select `bool` (>= _returnvalue_2 300.0) :`false` (select `bool` (>= _returnvalue_2 200.0) :`false` 90.0 :`true` 70.0 :!type "Float (single-precision)") :`true` 50.0) :`true` 30.0) "NewEnumerator2" _returnvalue null true)
          (break))))
    (:`Remote`
      _))
  (`GameplayStatics.PlayWorldCameraShake` "/Game/FirstPersonBP/Blueprints/FusionCoreShake.FusionCoreShake_C" _returnvalue 0.0 1000.0 1.0)
  (`KismetSystemLibrary.Delay` 0.1)
  (`self.K2_DestroyActor`)
  (set `self.Exploding` false))

(event `self.ReceiveBeginPlay`
  (bind _colorcenter (`self.ColorCenter`))
  ;[1 1 1] Changes Color of Material
  (bind _returnvalue (`PrimitiveComponent.CreateDynamicMaterialInstance` _colorcenter 0 (`PrimitiveComponent.GetMaterial` _colorcenter 0)))
  (bind _output_get (set `self.ColorCenterToChange` _returnvalue))
  (`PrimitiveComponent.SetMaterial` _colorcenter 0 _output_get))

(event `ReplicatedSound`
  (params (Sound :type "SoundBase Object Reference"))
  ;[1 1 1] Replication Stuff
  (`GameplayStatics.PlaySoundAtLocation` Sound (`self.K2_GetActorLocation`) (struct) 1.0 1.0 0.0 (`self.BlinkAttenuation`)))

(event `ReplicateBlink`
  (params (A :type "Float (double-precision)"))
  ;[1 1 1] Replication Stuff
  (`MaterialInstanceDynamic.SetVectorParameterValue` (`self.ColorCenterToChange`) "FusionCoreColor" (`KismetMathLibrary.LinearColorLerp` (struct :`G` 0.666 :`B` 1.0 :`A` 1.0) (struct :`R` 1.0 :`A` 1.0) (* A (`self.FlashSpeed`)))))

(event `ReplicatedEmitter`
  (params (EmitterTemplate :type "ParticleSystem Object Reference") (Sound :type "SoundBase Object Reference"))
  (bind _returnvalue (`self.K2_GetActorLocation`))
  ;[1 1 1] Replication Stuff
  (bind _returnvalue_2 (`GameplayStatics.SpawnEmitterAtLocation` EmitterTemplate _returnvalue))
  (`GameplayStatics.PlaySoundAtLocation` Sound _returnvalue)
  (`SceneComponent.SetWorldScale3D` _returnvalue_2 (5.0 5.0 5.0)))

(fn `FusionCoreDamage`
  (bind _fusioncorehealth (`self.FusionCoreHealth`))
  ;[1 1 1] Changes the Color of the ColorCenter on the Fusion Core
  (if (not (`self.Exploding`))
    (`MaterialInstanceDynamic.SetVectorParameterValue` (`self.ColorCenterToChange`) "FusionCoreColor" (`KismetMathLibrary.LinearColorLerp` (struct :`R` 1.0 :`A` 1.0) (struct :`G` 0.666 :`B` 1.0 :`A` 1.0) (/ (`/Game/FirstPersonBP/Blueprints/ActorComponents/HealthComponent.CurHealth` _fusioncorehealth) (`KismetMathLibrary.Conv_IntToDouble` (`/Game/FirstPersonBP/Blueprints/ActorComponents/HealthComponent.MaxHealth` _fusioncorehealth)))))))

(fn `UserConstructionScript`
  (bind _returnvalue (`PrimitiveComponent.CreateDynamicMaterialInstance` (`self.ColorCenter`) 0 null))
  (set `self.ColorCenterToChange` _returnvalue))