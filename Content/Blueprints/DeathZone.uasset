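; DeathZone is a boundary box that threatens the locally controlled first-person character with death after they leave it.
; Ending overlap starts a KillPlayer timer on the character's TimerComponent and, unless the game is over, flags the health component and fades in a warning widget.
; Re-entering clears the timer, flag and widget.
; The construction script gives the box a dynamic fire material.
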(event `self.Box.OnComponentEndOverlap`
  (params (OverlappedComponent :type "PrimitiveComponent Object Reference") (OtherActor :type "Actor Object Reference") (OtherComp :type "PrimitiveComponent Object Reference") (OtherBodyIndex :type Integer))
  (bind _asfirst_person_character (cast `/Game/FirstPersonBP/Blueprints/FirstPersonCharacter` OtherActor))
  (bind _returnvalue (`Pawn.GetController` _asfirst_person_character))
  (`/Engine/EditorBlueprintResources/StandardMacros.IsValid` _returnvalue
    (:`Is Valid`
      (if (`Controller.IsLocalPlayerController` _returnvalue)
        (bind _output_get (set `self.MyCharacter` _asfirst_person_character))
        (set `self.MyHealth` (`/Game/FirstPersonBP/Blueprints/FirstPersonCharacter.PlayerHealthComponent` _output_get))
        (bind _timercomponent (`/Game/FirstPersonBP/Blueprints/FirstPersonCharacter.TimerComponent` _output_get))
        (`KismetSystemLibrary.K2_SetTimer` _timercomponent "KillPlayer" (`/Game/FirstPersonBP/Blueprints/ActorComponents/TimerComponent.KillPlayerTimer` _timercomponent))
        (`self.OutsideTrigger`)))))

(event `self.Box.OnComponentBeginOverlap`
  (params (OverlappedComponent :type "PrimitiveComponent Object Reference") (OtherActor :type "Actor Object Reference") (OtherComp :type "PrimitiveComponent Object Reference") (OtherBodyIndex :type Integer) (bFromSweep :type Boolean) (SweepResult :type "HitResult Structure (by ref)"))
  (bind _asfirst_person_character (cast `/Game/FirstPersonBP/Blueprints/FirstPersonCharacter` OtherActor))
  (bind _returnvalue (`Pawn.GetController` _asfirst_person_character))
  (`/Engine/EditorBlueprintResources/StandardMacros.IsValid` _returnvalue
    (:`Is Valid`
      (if (`Controller.IsLocalPlayerController` _returnvalue)
        (set `self.MyCharacter` _asfirst_person_character)
        (`self.InsideTrigger`)))))

(event `OutsideTrigger`
  (if (not (`/Game/Networking/Blueprints/Gameplay/GameplayGM.GameOver` (cast `/Game/Networking/Blueprints/Gameplay/GameplayGM` (`GameplayStatics.GetGameMode`) :!pure true)))
    (set `self.CanDie` true)
    (bind _returnvalue (`|CreateWidget` "/Game/Networking/UI/Gameplay/DeathZoneUI.DeathZoneUI_C" (cast `/Game/Networking/Blueprints/Gameplay/GameplayPC` (`GameplayStatics.GetPlayerController` 0) :!pure true)))
    (bind _output_get (set `self.DeathZoneUI` _returnvalue))
    (set `/Game/FirstPersonBP/Blueprints/ActorComponents/HealthComponent.DeathZoneVisibility` true (`self.MyHealth`))
    (`UserWidget.AddToViewport` _output_get 0)
    (if (`self.CanDie`)
      (`/Game/Networking/UI/Gameplay/DeathZoneUI.StartDeathUIFadeIn` _output_get))))

(event `InsideTrigger`
  (bind _deathzoneui (`self.DeathZoneUI`))
  (bind _myhealth (`self.MyHealth`))
  (bind _mycharacter (`self.MyCharacter`))
  (set `self.CanDie` false)
  (`/Engine/EditorBlueprintResources/StandardMacros.IsValid` _myhealth
    (:`Is Valid`
      (set `/Game/FirstPersonBP/Blueprints/ActorComponents/HealthComponent.DeathZoneVisibility` false _myhealth)
      (`/Engine/EditorBlueprintResources/StandardMacros.IsValid` _mycharacter
        (:`Is Valid`
          (`KismetSystemLibrary.K2_ClearTimer` (`/Game/FirstPersonBP/Blueprints/FirstPersonCharacter.TimerComponent` _mycharacter) "KillPlayer"))
        (:`Is Not Valid`
          _)))
    (:`Is Not Valid`
      _))
  (`/Engine/EditorBlueprintResources/StandardMacros.IsValid` _deathzoneui
    (:`Is Valid`
      (`Widget.RemoveFromParent` _deathzoneui))))

(fn `UserConstructionScript`
  (`PrimitiveComponent.CreateDynamicMaterialInstance` (`self.Box`) 0 "/Game/AvdMagick/Materials/M_ky_fire01_4x8.M_ky_fire01_4x8"))